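; Game mode for an infinite terrain game that builds the starting run of tiles and tracks the score.
; On BeginPlay it calls FindBoundsVolume, then spawns a few BP_Tile actors in a chain.
; SpawnTile hands each tile the NavVolumePool and takes its attach location as the next tile's spawn transform.
; NewTileConquered only increments Score; it does not spawn further tiles.
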(event EventBeginPlay
  (Class|InfiniteTerrainGameMode|FindBoundsVolume)
  (for _index (range 0 3)
    (CallFunction|SpawnTile)))

(fn ConstructionScript)

(fn SpawnTile
  (bind _returnvalue (Game|SpawnActorfromClass "/Game/Dynamic/Terrain/BP_Tile.BP_Tile_C" (Variables|Default|GetNextTileTransform) "AlwaysSpawn" 0 0))
  (Class|Tile|SetPool _returnvalue (Variables|Default|GetNavVolumePool))
  (bind _attachtransform (Default|GetAttachLocation _returnvalue))
  (Variables|Default|SetNextTileTransform _attachtransform))

(fn NewTileConquered
  (Math|Integer|IncrementInt (Variables|Default|GetScore)))