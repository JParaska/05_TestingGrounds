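; Terrain tile for an infinite terrain game that scatters random counts of props and rocks on BeginPlay.
; Its barrier starts solid red, turns passable green while the player overlaps LockingVolume, then relocks on exit and asks InfiniteTerrainGameMode to spawn another tile.
; The player entering DestroyVolume destroys the tile.
; GetAttachLocation exposes the Arrow's world transform as an attach point.
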(event OnComponentEndOverlap(LockingVolume)
  (params (OverlappedComponent :type Primitive%20Component%20Object%20Reference) (OtherActor :type Actor%20Object%20Reference) (OtherComp :type Primitive%20Component%20Object%20Reference) (OtherBodyIndex :type Integer))
  (Utilities|IsPlayer OtherActor)
  (CallFunction|Lock)
  (bind _asinfinite_terrain_game_mode (Utilities|Casting|CastToInfiniteTerrainGameMode (Game|GetGameMode)))
  (Default|SpawnTile _asinfinite_terrain_game_mode))

(event OnComponentBeginOverlap(LockingVolume)
  (params (OverlappedComponent :type Primitive%20Component%20Object%20Reference) (OtherActor :type Actor%20Object%20Reference) (OtherComp :type Primitive%20Component%20Object%20Reference) (OtherBodyIndex :type Integer) (bFromSweep :type Boolean) (SweepResult :type Hit%20Result%20Structure%20%28by%20ref%29))
  (Utilities|IsPlayer OtherActor)
  (CallFunction|Unlock))

(event OnComponentBeginOverlap(DestroyVolume)
  (params (OverlappedComponent :type Primitive%20Component%20Object%20Reference) (OtherActor :type Actor%20Object%20Reference) (OtherComp :type Primitive%20Component%20Object%20Reference) (OtherBodyIndex :type Integer) (bFromSweep :type Boolean) (SweepResult :type Hit%20Result%20Structure%20%28by%20ref%29))
  (Utilities|IsPlayer OtherActor)
  (Actor|DestroyActor))

(event EventBeginPlay
  (CallFunction|Lock)
  (Class|Tile|PlaceActors "/Game/Dynamic/Terrain/Props/BP_Container.BP_Container_C" 1 3)
  (Class|Tile|PlaceActors "/Game/Dynamic/Terrain/Props/BP_Box.BP_Box_C" 2 4)
  (Class|Tile|PlaceActors "/Game/Dynamic/Terrain/Props/BP_Canister.BP_Canister_C" 3 5)
  (Class|Tile|PlaceActors "/Game/Dynamic/Terrain/Props/BP_SandBags.BP_SandBags_C" 1 2)
  (Class|Tile|PlaceActors "/Game/Dynamic/Terrain/Props/BP_Rock01.BP_Rock01_C" 1 4)
  (Class|Tile|PlaceActors "/Game/Dynamic/Terrain/Props/BP_Rock02.BP_Rock02_C" 1 4)
  (Class|Tile|PlaceActors "/Game/Dynamic/Terrain/Props/BP_Rock03.BP_Rock03_C" 1 4))

(fn ConstructionScript)

(fn GetAttachLocation
  (return (Transformation|GetWorldTransform (Variables|Default|GetArrow))))

(fn Unlock
  (bind _barrier (Variables|Default|GetBarrier))
  (Collision|SetCollisionEnabled _barrier "NoCollision")
  (Rendering|Material|SetMaterial _barrier 0 "/Game/Dynamic/Terrain/MI_Barrier_Green.MI_Barrier_Green"))

(fn Lock
  (bind _barrier (Variables|Default|GetBarrier))
  (Collision|SetCollisionEnabled _barrier "QueryAndPhysics")
  (Rendering|Material|SetMaterial _barrier 0 "/Game/Dynamic/Terrain/MI_Barrier_Red.MI_Barrier_Red"))